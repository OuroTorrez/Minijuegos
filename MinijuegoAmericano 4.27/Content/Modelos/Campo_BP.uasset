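; Field Blueprint that spawns escalating waves of Tackler AI at random spawn points across the field.
; After an initial delay and first spawn, an endless delayed loop calls SpawnTacklers, raising the spawn amount every fourth wave.
; Each call rebuilds the array of spawn components and removes a random entry after each spawn, re-rolled so not necessarily the point just used.
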(event Custom|SpawnTacklers
  (params (NewParam :type Integer))
  (bind _array (CallFunction|MakeSpawnerArray))
  (bind _output_get (Variables|Spawner|SetSpawnerArray _array))
  (for _index (range 0 NewParam)
    (AI|SpawnAIFromClass "/Game/ThirdPersonBP/Blueprints/Tackler.Tackler_C" 0 (Transformation|GetWorldLocation (.OutItem (Utilities|Array|Random _output_get))) (Transformation|GetWorldRotation (.OutItem (Utilities|Array|Random _output_get))) false 0)
    (Utilities|Array|RemoveItem _output_get (.OutItem (Utilities|Array|Random _output_get)))))

(event EventBeginPlay
  (Utilities|FlowControl|Delay 6.0)
  (CallFunction|SpawnTacklers 1)
  (Utilities|FlowControl|Delay 2.0 :!label _label)
  (CallFunction|SpawnTacklers (Variables|Default|GetSpawnAmount))
  (bind _output_get (Variables|Default|SetTimes (+ (Variables|Default|GetTimes) 1)))
  (if (== _output_get 4)
    (Variables|Default|SetSpawnAmount (+ (Variables|Default|GetSpawnAmount) 1))
    (Variables|Default|SetTimes 0)
    (goto _label)
    (else
      (goto _label))))

(event Collision|EventActorBeginOverlap
  (params (OtherActor :type Actor%20Object%20Reference)))

(event EventTick
  (params (DeltaSeconds :type Float%20%28single-precision%29)))

(fn ConstructionScript)

(fn MakeSpawnerArray
  (return (Utilities|Array|MakeArray (Variables|Spawner|GetSpawn) (Variables|Spawner|GetSpawn1) (Variables|Spawner|GetSpawn2) (Variables|Spawner|GetSpawn3) (Variables|Spawner|GetSpawn4) (Variables|Spawner|GetSpawn5) (Variables|Spawner|GetSpawn6) (Variables|Spawner|GetSpawn7) (Variables|Spawner|GetSpawn8) (Variables|Spawner|GetSpawn9) (Variables|Spawner|GetSpawn10) (Variables|Spawner|GetSpawn11) (Variables|Spawner|GetSpawn12) (Variables|Spawner|GetSpawn13) (Variables|Spawner|GetSpawn14))))