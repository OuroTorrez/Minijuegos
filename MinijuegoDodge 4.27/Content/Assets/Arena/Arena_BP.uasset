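; Arena actor that spawns cannons and coins and explodes Projectile2_BP projectiles when they leave its sphere.
; After a startup delay, a timed loop spawns Cannon_BP at random navmesh points near the center until the count reaches its limit.
; While CanSpawnCoins is set, a Tick accumulator triggers periodic Coin_BP waves over a wider radius, with wave size growing to a cap.
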(event OnComponentEndOverlap(Sphere)
  (params (OverlappedComponent :type Primitive%20Component%20Object%20Reference) (OtherActor :type Actor%20Object%20Reference) (OtherComp :type Primitive%20Component%20Object%20Reference) (OtherBodyIndex :type Integer))
  (bind _asprojectile_2_bp (Utilities|Casting|CastToProjectile2_BP OtherActor))
  (Default|Explode _asprojectile_2_bp))

(event Custom|SpawnCannons
  (bind _defaultsceneroot (Variables|Default|GetDefaultSceneRoot))
  (bind _returnvalue (Transformation|GetWorldLocation _defaultsceneroot))
  (bind _randomlocation (Class|NavigationSystemV1|GetRandomPointinNavigableRadius _returnvalue 3e+02 0 0))
  (Utilities|FlowControl|Delay 4.0)
  (Game|SpawnActorfromClass "/Game/Assets/Cannon/Cannon_BP.Cannon_BP_C" (Math|Transform|MakeTransform (Math|Vector|MakeVector (.x _randomlocation) (.y _randomlocation) 3e+02) "0, 0, 0" "1,1,1") "Undefined" 0 "0.000000,0.000000,0.000000" "0.000000,0.000000,0.000000" 0 :!label _label)
  (Variables|Default|SetCannonObjs (+ (Variables|Default|GetCannonObjs) 1.0))
  (Utilities|FlowControl|Delay 1e+01)
  (if (< (Variables|Default|GetCannonObjs) 3.0)
    (goto _label)))

(event Custom|SpawnCoins
  (bind _defaultsceneroot (Variables|Default|GetDefaultSceneRoot))
  (bind _returnvalue (Transformation|GetWorldLocation _defaultsceneroot))
  (bind _randomlocation (Class|NavigationSystemV1|GetRandomPointinNavigableRadius _returnvalue 6e+02 0 0))
  (for _index (range 0 (Variables|Default|GetCoinsObjs))
    (Game|SpawnActorfromClass "/Game/Assets/Coin/Coin_BP.Coin_BP_C" (Math|Transform|MakeTransform (Math|Vector|MakeVector (.x _randomlocation) (.y _randomlocation) 1e+01) "0, 0, 0" "1,1,1") "Undefined" 0 0))
  (if (< (Variables|Default|GetCoinsObjs) 9)
    (Variables|Default|SetCoinsObjs (+ (Variables|Default|GetCoinsObjs) 3))))

(event EventBeginPlay
  (CallFunction|SpawnCannons))

(event Collision|EventActorBeginOverlap
  (params (OtherActor :type Actor%20Object%20Reference)))

(event EventTick
  (params (DeltaSeconds :type Float%20%28single-precision%29))
  (if (Variables|Default|GetcanSpawnCoins)
    (Variables|Default|SetDeltaSpawnCoinRate (+ (Variables|Default|GetDeltaSpawnCoinRate) DeltaSeconds))
    (if (>= (Variables|Default|GetDeltaSpawnCoinRate) (Variables|Default|GetSpawnCoinRate))
      (Variables|Default|SetDeltaSpawnCoinRate 0.0)
      (CallFunction|SpawnCoins))))

(fn ConstructionScript)