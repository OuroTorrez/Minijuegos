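; Electric stun projectile actor that stuns the ThirdPerson player or bot character it hits.
; The construction script builds a relative two-point InterpToMovement path ending 2000 units along X, timed by the Duration variable.
; BeginPlay attaches looping-style spark and voltage effects to the Projectile component.
; A hit on either character calls Stunned, then Explode spawns spark bursts and sounds and destroys the actor; other hits are ignored.
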(event EventBeginPlay
  (bind _returnvalue (Audio|SpawnSoundAttached "/Game/Assets/Projectile/Electricity_Voltage.Electricity_Voltage" (Variables|Default|GetProjectile) "None" "0, 0, 0" "0, 0, 0" "KeepRelativeOffset" true 0.2 1.0 0.0 0 0 false))
  (Variables|Default|SetSound _returnvalue)
  (Effects|SpawnEmitterAttached "/Game/StarterContent/Particles/P_Sparks.P_Sparks" (Variables|Default|GetProjectile) "None"))

(event Collision|EventActorBeginOverlap
  (params (OtherActor :type Actor%20Object%20Reference)))

(event EventTick
  (params (DeltaSeconds :type Float%20%28single-precision%29)))

(event Collision|EventHit
  (params (MyComp :type Primitive%20Component%20Object%20Reference) (Other :type Actor%20Object%20Reference) (OtherComp :type Primitive%20Component%20Object%20Reference) (bSelfMoved :type Boolean) (HitLocation :type Vector :default "0, 0, 0") (HitNormal :type Vector :default "0, 0, 0") (NormalImpulse :type Vector :default "0, 0, 0") (Hit :type Hit%20Result%20Structure%20%28by%20ref%29))
  (bind _asthird_person_character (Utilities|Casting|CastToThirdPersonCharacter Other)
    (:then
      (Default|Stunned _asthird_person_character)
      (CallFunction|Explode))
    (:CastFailed
      (bind _asthird_person_bot_character (Utilities|Casting|CastToThirdPersonBotCharacter Other))
      (Default|Stunned _asthird_person_bot_character)
      (CallFunction|Explode))))

(fn ConstructionScript
  (bind (_x _y _z) (Math|Vector|BreakVector "0, 0, 0"))
  (bind _interptomovement (Variables|Default|GetInterpToMovement))
  (Variables|Default|SetLocation2 (Math|Vector|MakeVector (+ _x 2e+03) _y _z))
  (Variables|/Script/Engine.InterpToMovementComponent|SetControlPoints _interptomovement (Utilities|Array|MakeArray (Utilities|Struct|MakeInterpControlPoint (Variables|Default|GetLocation1) true) (Utilities|Struct|MakeInterpControlPoint (Variables|Default|GetLocation2) true)))
  (Variables|/Script/Engine.InterpToMovementComponent|SetDuration _interptomovement (Variables|Default|GetDuration)))

(fn Explode
  (bind _returnvalue (Transformation|GetActorLocation))
  (Effects|SpawnEmitteratLocation "/Game/InfinityBladeEffects/Effects/FX_Monsters/FX_Monster_Genno/P_Genno_WeaponDrag_Sparks_01.P_Genno_WeaponDrag_Sparks_01" _returnvalue)
  (Effects|SpawnEmitteratLocation "/Game/InfinityBladeEffects/Effects/FX_Monsters/FX_Monster_GolemBot/Notifies/P_SparkBurst.P_SparkBurst" _returnvalue)
  (Audio|PlaySoundatLocation "/Game/StarterContent/Audio/Explosion01.Explosion01" _returnvalue "0, 0, 0" 0.1 1.0 0.0 0 0 0)
  (Audio|PlaySoundatLocation "/Game/Assets/Projectile/Electric_Zap.Electric_Zap" "0, 0, 0" "0, 0, 0" 0.2 1.0 0.0 0 0 0)
  (Actor|DestroyActor))