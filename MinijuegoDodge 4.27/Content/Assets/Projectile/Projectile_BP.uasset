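; Electric projectile actor that stuns the player or bot character it hits, then explodes with sparks and a zap sound.
; Construction sets up an InterpToMovement path ending 300 units down, and BeginPlay attaches sparks and a looping-style voltage sound.
; If still alive after half a second, it picks one of four random axes, spawns two Projectile2_BP actors facing opposite ways along it, and destroys itself.
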(event EventBeginPlay
  (bind _returnvalue (Audio|SpawnSoundAttached "/Game/Assets/Projectile/Electricity_Voltage.Electricity_Voltage" (Variables|Default|GetProjectile) "None" "0, 0, 0" "0, 0, 0" "KeepWorldPosition" true 0.2 1.0 0.0 0 0 false))
  (Variables|Default|SetSound _returnvalue)
  (Effects|SpawnEmitterAttached "/Game/StarterContent/Particles/P_Sparks.P_Sparks" (Variables|Default|GetProjectile) "None")
  (Utilities|FlowControl|Delay 0.5)
  (switch int (Math|Random|RandomInteger 4)
    (:0
      (CallFunction|GetDirection "0, 0, 0" "0,-180.000000, 0"))
    (:1
      (CallFunction|GetDirection "0,90.000000, 0" "0.000000,-90.000000, 0"))
    (:2
      (CallFunction|GetDirection "0,-45.000000, 0" "0.000000,135.000000,0.000000"))
    (:3
      (CallFunction|GetDirection "0,45.000000, 0" "0.000000,-135.000000,0.000000")))
  (Actor|DestroyActor))

(event Collision|EventActorBeginOverlap
  (params (OtherActor :type Actor%20Object%20Reference)))

(event EventTick
  (params (DeltaSeconds :type Float%20%28single-precision%29)))

(event Collision|EventHit
  (params (MyComp :type Primitive%20Component%20Object%20Reference) (Other :type Actor%20Object%20Reference) (OtherComp :type Primitive%20Component%20Object%20Reference) (bSelfMoved :type Boolean) (HitLocation :type Vector :default "0, 0, 0") (HitNormal :type Vector :default "0, 0, 0") (NormalImpulse :type Vector :default "0, 0, 0") (Hit :type Hit%20Result%20Structure%20%28by%20ref%29))
  (bind _asthird_person_character (Utilities|Casting|CastToThirdPersonCharacter Other)
    (:then
      (Default|Stunned _asthird_person_character)
      (CallFunction|Explode))
    (:CastFailed
      (bind _asthird_person_bot_character (Utilities|Casting|CastToThirdPersonBotCharacter Other))
      (Default|Stunned _asthird_person_bot_character)
      (CallFunction|Explode))))

(fn ConstructionScript
  (bind (_x _y _z) (Math|Vector|BreakVector "0, 0, 0"))
  (bind _interptomovement (Variables|Default|GetInterpToMovement))
  (Variables|Default|SetLocation2 (Math|Vector|MakeVector _x _y (- _z 3e+02)))
  (Variables|/Script/Engine.InterpToMovementComponent|SetControlPoints _interptomovement (Utilities|Array|MakeArray (Utilities|Struct|MakeInterpControlPoint (Variables|Default|GetLocation1) true) (Utilities|Struct|MakeInterpControlPoint (Variables|Default|GetLocation2) true)))
  (Variables|/Script/Engine.InterpToMovementComponent|SetDuration _interptomovement (Variables|Default|GetDuration)))

(fn GetDirection
  (params (Spawn%20Transform%20Rotation :type Rotator) (Spawn%20Transform%20Rotation1 :type Rotator))
  (bind _returnvalue (Transformation|GetActorLocation))
  (Game|SpawnActorfromClass "/Game/Assets/Projectile/Projectile2_BP.Projectile2_BP_C" (Math|Transform|MakeTransform _returnvalue Spawn%20Transform%20Rotation "1,1,1") "Undefined" 0 0)
  (Game|SpawnActorfromClass "/Game/Assets/Projectile/Projectile2_BP.Projectile2_BP_C" (Math|Transform|MakeTransform _returnvalue Spawn%20Transform%20Rotation1 "1,1,1") "Undefined" 0 0))

(fn Explode
  (bind _returnvalue (Transformation|GetActorLocation))
  (Effects|SpawnEmitteratLocation "/Game/InfinityBladeEffects/Effects/FX_Monsters/FX_Monster_Genno/P_Genno_WeaponDrag_Sparks_01.P_Genno_WeaponDrag_Sparks_01" _returnvalue)
  (Effects|SpawnEmitteratLocation "/Game/InfinityBladeEffects/Effects/FX_Monsters/FX_Monster_GolemBot/Notifies/P_SparkBurst.P_SparkBurst" _returnvalue)
  (Audio|PlaySoundatLocation "/Game/Assets/Projectile/Electric_Zap.Electric_Zap" _returnvalue "0, 0, 0" 0.2 1.0 0.0 0 0 0)
  (Actor|DestroyActor))