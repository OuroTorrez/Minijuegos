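; Coin pickup actor that the third-person player or bot character collects by touching it.
; On sphere overlap it casts the other actor to ThirdPersonCharacter, falling back to ThirdPersonBotCharacter, and adds one to that character's Coins.
; Either path then calls GetCoin, which plays a quiet pickup sound, spawns a particle effect at the coin's location and destroys the actor.
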(event OnComponentBeginOverlap(Sphere)
  (params (OverlappedComponent :type Primitive%20Component%20Object%20Reference) (OtherActor :type Actor%20Object%20Reference) (OtherComp :type Primitive%20Component%20Object%20Reference) (OtherBodyIndex :type Integer) (bFromSweep :type Boolean) (SweepResult :type Hit%20Result%20Structure%20%28by%20ref%29))
  (bind _asthird_person_character (Utilities|Casting|CastToThirdPersonCharacter OtherActor)
    (:then
      (Variables|/Game/ThirdPersonBP/Blueprints/ThirdPersonCharacter.ThirdPersonCharacter_C|SetCoins _asthird_person_character (+ (Variables|/Game/ThirdPersonBP/Blueprints/ThirdPersonCharacter.ThirdPersonCharacter_C|GetCoins _asthird_person_character) 1)))
    (:CastFailed
      (bind _asthird_person_bot_character (Utilities|Casting|CastToThirdPersonBotCharacter OtherActor))
      (Variables|/Game/ThirdPersonBP/Blueprints/ThirdPersonBotCharacter.ThirdPersonBotCharacter_C|SetCoins _asthird_person_bot_character (+ (Variables|/Game/ThirdPersonBP/Blueprints/ThirdPersonBotCharacter.ThirdPersonBotCharacter_C|GetCoins _asthird_person_bot_character) 1))))
  (CallFunction|GetCoin))

(event EventBeginPlay)

(event Collision|EventActorBeginOverlap
  (params (OtherActor :type Actor%20Object%20Reference)))

(event EventTick
  (params (DeltaSeconds :type Float%20%28single-precision%29)))

(fn ConstructionScript)

(fn GetCoin
  (bind _returnvalue (Transformation|GetActorLocation))
  (Audio|PlaySoundatLocation "/Game/Assets/Coin/PickCoin.PickCoin" _returnvalue "0, 0, 0" 0.2 1.0 0.0 0 0 0)
  (Effects|SpawnEmitteratLocation "/Game/InfinityBladeEffects/Effects/FX_Treasure/Loot/P_KeyPickup_01.P_KeyPickup_01" _returnvalue)
  (Actor|DestroyActor))