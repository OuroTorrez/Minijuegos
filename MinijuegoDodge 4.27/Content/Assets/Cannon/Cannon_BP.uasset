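; Hovering cannon actor that repeatedly waits, spawns a Projectile_BP, then glides to a random navigable point nearby until EndFiring is set.
; While waiting to fire, Tick draws a red downward debug trace as an aiming line, without using the hit result.
; Once EndFiring and EndMove are true, Tick sends it on a single higher, randomized exit move.
; The construction script builds two vertically offset InterpToMovement control points using Duration.
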(event EventBeginPlay
  (bind _defaultsceneroot (Variables|Default|GetDefaultSceneRoot))
  (Variables|Default|SetWaitingToFire true :!label _label)
  (Utilities|FlowControl|Delay 3.0)
  (Game|SpawnActorfromClass "/Game/Assets/Projectile/Projectile_BP.Projectile_BP_C" (Math|Transform|MakeTransform (Transformation|GetWorldLocation (Variables|Default|GetDefaultSceneRoot)) "0, 0, 0" "1,1,1") "Undefined" 0 0)
  (Variables|Default|SetWaitingToFire false)
  (bind _randomlocation (Class|NavigationSystemV1|GetRandomLocationinNavigableRadius (Transformation|GetWorldLocation _defaultsceneroot) 1e+03 0 0))
  (Components|MoveComponentTo _defaultsceneroot (Math|Vector|MakeVector (.x _randomlocation) (.y _randomlocation) 3.5e+02) "0, 0, 0" true true 3.0 false)
  (if (not (Variables|Default|GetEndFiring))
    (goto _label)))

(event Collision|EventActorBeginOverlap
  (params (OtherActor :type Actor%20Object%20Reference)))

(event EventTick
  (params (DeltaSeconds :type Float%20%28single-precision%29))
  (bind _defaultsceneroot (Variables|Default|GetDefaultSceneRoot))
  (bind _defaultsceneroot_2 (Variables|Default|GetDefaultSceneRoot))
  (bind _returnvalue (Transformation|GetWorldLocation _defaultsceneroot))
  (bind _returnvalue_2 (Transformation|GetWorldLocation _defaultsceneroot_2))
  (if (Variables|Default|GetEndFiring)
    (if (Variables|Default|GetendMove)
      (Variables|Default|SetendMove false)
      (Components|MoveComponentTo _defaultsceneroot_2 (Math|Vector|MakeVector (Math|Random|RandomFloatinRange (.x _returnvalue_2) 1e+04) (Math|Random|RandomFloatinRange (.y _returnvalue_2) 1e+04) 1e+03) "0, 0, 0" true true 5.0 false))
    (elif (Variables|Default|GetWaitingToFire)
      (Collision|LineTraceByChannel _returnvalue (+ _returnvalue (* (Math|Vector|GetUpVector (Transformation|GetWorldRotation _defaultsceneroot)) -1e+03)) "TraceTypeQuery2" false 0 "ForOneFrame" true "(R=1.000000,G=0.000000,B=0.000000,A=0.000000)"))))

(fn ConstructionScript
  (bind _defaultsceneroot (Variables|Default|GetDefaultSceneRoot))
  (bind _interptomovement (Variables|Default|GetInterpToMovement))
  (bind _returnvalue (Transformation|GetWorldLocation _defaultsceneroot))
  (bind (_x _y _z) (Math|Vector|BreakVector _returnvalue))
  (Variables|Default|SetLocation1 _returnvalue)
  (Variables|Default|SetLocation2 (Math|Vector|MakeVector _x _y (- _z 2.5e+02)))
  (Variables|/Script/Engine.InterpToMovementComponent|SetControlPoints _interptomovement (Utilities|Array|MakeArray (Utilities|Struct|MakeInterpControlPoint (Variables|Default|GetLocation1) true) (Utilities|Struct|MakeInterpControlPoint (Variables|Default|GetLocation2) true)))
  (Variables|/Script/Engine.InterpToMovementComponent|SetDuration _interptomovement (Variables|Default|GetDuration)))